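; BP_Weapon is a melee weapon actor that detects hits during swings and bashes and passes them to the struck character.
; While tracing, Tick sweeps spheres from last-frame to current socket positions: start, midpoint and end for swings, one for bashes.
; Each actor registers once per swing; third-person characters receive the owner's current attack data via ReceiveAttack.
; Bash tracing seeds from Trace_Bash but updates from Trace_Start.
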(event EventBeginPlay)

(event Collision|EventActorBeginOverlap
  (params (OtherActor :type Actor%20Object%20Reference)))

(event EventTick
  (params (DeltaSeconds :type Float%20%28single-precision%29))
  (if (Variables|Default|GetIsTracing)
    (CallFunction|UpdateWeaponTrace)
    (elif (Variables|Default|GetIsTracingBash)
      (CallFunction|UpdateBashTrace))))

(fn ConstructionScript)

(fn StartWeaponTrace
  (Utilities|Array|Clear (Variables|Default|GetHitActorsThisSwing))
  (Variables|Default|SetIsTracing true)
  (Variables|Default|SetPreviousStart (Transformation|GetSocketLocation (Variables|Default|GetWeaponMesh) "Trace_Start"))
  (Variables|Default|SetPreviousEnd (Transformation|GetSocketLocation (Variables|Default|GetWeaponMesh) "Trace_End")))

(fn StopWeaponTrace
  (Variables|Default|SetIsTracing false)
  (Variables|Default|SetIsTracingBash false))

(fn UpdateWeaponTrace
  (bind _weaponmesh (Variables|Default|GetWeaponMesh))
  (bind _output_get (LocalVariables|SetCurrentStart (Transformation|GetSocketLocation _weaponmesh "Trace_Start")))
  (bind _output_get_2 (LocalVariables|SetCurrentEnd (Transformation|GetSocketLocation _weaponmesh "Trace_End")))
  (LocalVariables|SetPreviousMid (Math|Vector|Lerp(Vector) (Variables|Default|GetPreviousStart) (Variables|Default|GetPreviousEnd) 0.5))
  (LocalVariables|SetCurrentMid (Math|Vector|Lerp(Vector) _output_get _output_get_2 0.5))
  (bind (_outhit _returnvalue) (Collision|SphereTraceByChannel (Variables|Default|GetPreviousStart) _output_get (Variables|Default|GetTraceRadius) "TraceTypeQuery2" false (Utilities|Array|MakeArray (Variables|Default|GetOwnerCharacter)) "None"))
  (CallFunction|HandleTraceHit _returnvalue _outhit)
  (bind (_outhit_2 _returnvalue_2) (Collision|SphereTraceByChannel (Variables|Default|GetPreviousEnd) (LocalVariables|GetCurrentEnd) (Variables|Default|GetTraceRadius) "TraceTypeQuery2" false (Utilities|Array|MakeArray (Variables|Default|GetOwnerCharacter)) "None"))
  (CallFunction|HandleTraceHit _returnvalue_2 _outhit_2)
  (bind (_outhit_3 _returnvalue_3) (Collision|SphereTraceByChannel (LocalVariables|GetPreviousMid) (LocalVariables|GetCurrentMid) (Variables|Default|GetTraceRadius) "TraceTypeQuery2" false (Utilities|Array|MakeArray (Variables|Default|GetOwnerCharacter)) "None"))
  (CallFunction|HandleTraceHit _returnvalue_3 _outhit_3)
  (Variables|Default|SetPreviousStart (LocalVariables|GetCurrentStart))
  (Variables|Default|SetPreviousEnd (LocalVariables|GetCurrentEnd)))

(fn ProcessHit
  (params (HitActor :type Actor%20Object%20Reference) (HitResult :type Hit%20Result%20Structure))
  (bind _ownercharacter (Variables|Default|GetOwnerCharacter))
  (bind _asbp_third_person_character (Utilities|Casting|CastToBP_ThirdPersonCharacter HitActor))
  (Default|ReceiveAttack _asbp_third_person_character _ownercharacter (Variables|/Game/ThirdPerson/Blueprints/BP_ThirdPersonCharacter.BP_ThirdPersonCharacter_C|GetCurrentAttackData _ownercharacter) HitResult))

(fn HandleTraceHit
  (params (DidHit :type Boolean) (HitResult :type Hit%20Result%20Structure))
  (bind _hitactor (Collision|BreakHitResult HitResult))
  (if DidHit
    (if (Utilities|IsValid _hitactor)
      (if (!= _hitactor (Variables|Default|GetOwnerCharacter))
        (if (not (Utilities|Array|ContainsItem (Variables|Default|GetHitActorsThisSwing) _hitactor))
          (Utilities|Array|Add (Variables|Default|GetHitActorsThisSwing) _hitactor)
          (CallFunction|ProcessHit _hitactor HitResult))))))

(fn StartBashTrace
  (Utilities|Array|Clear (Variables|Default|GetHitActorsThisSwing))
  (Variables|Default|SetIsTracingBash true)
  (Variables|Default|SetPreviousBash (Transformation|GetSocketLocation (Variables|Default|GetWeaponMesh) "Trace_Bash")))

(fn UpdateBashTrace
  (bind _output_get (LocalVariables|SetCurrentBash (Transformation|GetSocketLocation (Variables|Default|GetWeaponMesh) "Trace_Start")))
  (bind (_outhit _returnvalue) (Collision|SphereTraceByChannel (Variables|Default|GetPreviousBash) _output_get (Variables|Default|GetTraceRadius) "TraceTypeQuery2" false (Utilities|Array|MakeArray (Variables|Default|GetOwnerCharacter)) "None"))
  (CallFunction|HandleTraceHit _returnvalue _outhit)
  (Variables|Default|SetPreviousBash (LocalVariables|GetCurrentBash)))