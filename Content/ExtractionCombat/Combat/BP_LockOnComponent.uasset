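; Lock-on component for BP_ThirdPersonCharacter that toggles targeting of the nearest other character within LockRange.
; Targets come from sphere overlaps, and SwitchTarget cycles through them by axis sign with wraparound.
; Locking makes the owner face controller yaw and, for player-controlled owners, switches to the combat camera and shows guard indicators.
; Tick releases out-of-range targets, though release only succeeds in one specific AttackState.
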(event EventBeginPlay)

(event EventTick
  (params (DeltaSeconds :type Float%20%28single-precision%29))
  (if (Utilities|IsValid (Variables|Default|GetCurrentTarget))
    (if (> (Math|Vector|Distance(Vector) (Transformation|GetActorLocation (Components|GetOwner)) (Transformation|GetActorLocation (Variables|Default|GetCurrentTarget))) (Variables|Default|GetLockRange))
      (CallFunction|DeactivateLockon))))

(fn FindNearestTarget
  (bind _returnvalue (Components|GetOwner))
  (if (Variables|Default|GetIsLockedOn)
    (CallFunction|DeactivateLockon)
    (else
      (bind _ascharacter (Utilities|Casting|CastToCharacter _returnvalue))
      (bind _output_get (Variables|Default|SetOwnerCharacter _ascharacter))
      (Variables|Default|SetCurrentTarget 0)
      ;[0.15 0.15 0.15 0.5] Player´s Location
      (bind _output_get_2 (Variables|Default|SetOwnerLocation (Transformation|GetActorLocation _returnvalue)))
      (Variables|Default|SetClosestDistance (Variables|Default|GetLockRange))
      (bind _outactors (Collision|SphereOverlapActors (Transformation|GetActorLocation _output_get) (Variables|Default|GetLockRange) (Utilities|Array|MakeArray "ObjectTypeQuery3") "/Game/ThirdPerson/Blueprints/BP_ThirdPersonCharacter.BP_ThirdPersonCharacter_C" (Utilities|Array|MakeArray _output_get)))
      (for _array_element _outactors
        (if (!= (Variables|Default|GetOwnerCharacter) _array_element)
          (if (<= (Math|Vector|Distance(Vector) _output_get_2 (Transformation|GetActorLocation _array_element)) (Variables|Default|GetLockRange))
            (if (< (Math|Vector|Distance(Vector) _output_get_2 (Transformation|GetActorLocation _array_element)) (Variables|Default|GetClosestDistance))
              (Variables|Default|SetClosestDistance (Math|Vector|Distance(Vector) _output_get_2 (Transformation|GetActorLocation _array_element)))
              (if (Utilities|IsValid (Variables|Default|GetCurrentTarget))
                (bind _asbp_third_person_character (Utilities|Casting|CastToBP_ThirdPersonCharacter (Variables|Default|GetCurrentTarget)))
                (Default|SetEnemyGuardVisible _asbp_third_person_character false))
              (Variables|Default|SetCurrentTarget _array_element)
              (CallFunction|ActivateLockon))))))))

(fn ActivateLockon
  (bind _returnvalue (Components|GetOwner))
  (Variables|Default|SetIsLockedOn true)
  (bind _ascharacter (Utilities|Casting|CastToCharacter _returnvalue))
  (Variables|/Script/Engine.CharacterMovementComponent|SetbOrientRotationToMovement (Variables|/Script/Engine.Character|GetCharacterMovement _ascharacter) false)
  (Variables|/Script/Engine.Pawn|SetbUseControllerRotationYaw _ascharacter true)
  (bind _asbp_third_person_character (Utilities|Casting|CastToBP_ThirdPersonCharacter _returnvalue))
  (if (Pawn|IsPlayerControlled _asbp_third_person_character)
    (Default|CombatCamera _asbp_third_person_character)
    (Rendering|SetVisibility (Variables|/Game/ThirdPerson/Blueprints/BP_ThirdPersonCharacter.BP_ThirdPersonCharacter_C|GetGuardWidget _asbp_third_person_character) true false)
    (bind _aswbp_guard_indicator (Utilities|Casting|CastToWBP_GuardIndicator (UserInterface|GetUserWidgetObject (Variables|/Game/ThirdPerson/Blueprints/BP_ThirdPersonCharacter.BP_ThirdPersonCharacter_C|GetGuardWidget _asbp_third_person_character))))
    (Default|UpdateGuard _aswbp_guard_indicator (Variables|/Game/ThirdPerson/Blueprints/BP_ThirdPersonCharacter.BP_ThirdPersonCharacter_C|GetGuardDirection _asbp_third_person_character))
    (bind _asbp_third_person_character_2 (Utilities|Casting|CastToBP_ThirdPersonCharacter (Variables|Default|GetCurrentTarget)))
    (Default|SetEnemyGuardVisible _asbp_third_person_character_2 true)))

(fn DeactivateLockon
  (bind _returnvalue (Components|GetOwner))
  (bind _asbp_third_person_character (Utilities|Casting|CastToBP_ThirdPersonCharacter (Variables|Default|GetOwnerCharacter)))
  (if (Utilities|Enum|Equal(Enum) (Variables|/Game/ThirdPerson/Blueprints/BP_ThirdPersonCharacter.BP_ThirdPersonCharacter_C|GetAttackState _asbp_third_person_character) "NewEnumerator0")
    (Variables|Default|SetIsLockedOn false)
    (Variables|Default|SetClosestDistance 0.0)
    (bind _ascharacter (Utilities|Casting|CastToCharacter _returnvalue))
    (Variables|/Script/Engine.CharacterMovementComponent|SetbOrientRotationToMovement (Variables|/Script/Engine.Character|GetCharacterMovement _ascharacter) true)
    (Variables|/Script/Engine.Pawn|SetbUseControllerRotationYaw _ascharacter false)
    (bind _asbp_third_person_character_2 (Utilities|Casting|CastToBP_ThirdPersonCharacter _returnvalue))
    (if (Pawn|IsPlayerControlled _asbp_third_person_character_2)
      (Default|RestoreCamera _asbp_third_person_character_2)
      (Rendering|SetVisibility (Variables|/Game/ThirdPerson/Blueprints/BP_ThirdPersonCharacter.BP_ThirdPersonCharacter_C|GetGuardWidget _asbp_third_person_character_2) false false)
      (bind _asbp_third_person_character_3 (Utilities|Casting|CastToBP_ThirdPersonCharacter (Variables|Default|GetCurrentTarget)))
      (Default|SetEnemyGuardVisible _asbp_third_person_character_3 false)
      (Variables|Default|SetCurrentTarget 0)
      (else
        (Variables|Default|SetCurrentTarget 0)))))

(fn SwitchTarget
  (params (AxisValue%20 :type Float%20%28double-precision%29))
  (bind _targets_ (LocalVariables|GetTargets%20))
  (if (Utilities|IsValid (Variables|Default|GetCurrentTarget))
    (bind _output_get (LocalVariables|SetPlayerCharacter (Components|GetOwner)))
    (Utilities|Array|Clear (LocalVariables|GetTargets%20))
    (bind _outactors (Collision|SphereOverlapActors (Transformation|GetActorLocation _output_get) (Variables|Default|GetLockRange) (Utilities|Array|MakeArray "ObjectTypeQuery3") "/Game/ThirdPerson/Blueprints/BP_ThirdPersonCharacter.BP_ThirdPersonCharacter_C" (Utilities|Array|MakeArray _output_get)))
    (for _array_element _outactors
      (bind _asbp_third_person_character (Utilities|Casting|CastToBP_ThirdPersonCharacter _array_element))
      (Utilities|Array|Add (LocalVariables|GetTargets%20) _asbp_third_person_character))
    (if (> (Utilities|Array|Length _targets_) 0)
      (bind _asbp_third_person_character_2 (Utilities|Casting|CastToBP_ThirdPersonCharacter (Variables|Default|GetCurrentTarget)))
      (LocalVariables|SetTargetIndex (Utilities|Array|FindItem _targets_ _asbp_third_person_character_2))
      (if (> AxisValue%20 0.0)
        (LocalVariables|SetTargetIndex (+ (LocalVariables|GetTargetIndex) 1))
        (else
          (LocalVariables|SetTargetIndex (- (LocalVariables|GetTargetIndex) 1))))
      (if (>= (LocalVariables|GetTargetIndex) (Utilities|Array|Length (LocalVariables|GetTargets%20)))
        (LocalVariables|SetTargetIndex 0)
        (elif (< (LocalVariables|GetTargetIndex) 0)
          (LocalVariables|SetTargetIndex (- (Utilities|Array|Length (LocalVariables|GetTargets%20)) 1))))
      (bind _asbp_third_person_character_3 (Utilities|Casting|CastToBP_ThirdPersonCharacter (Variables|Default|GetCurrentTarget)))
      (Default|SetEnemyGuardVisible _asbp_third_person_character_3 false)
      (bind _output_get_2 (Variables|Default|SetCurrentTarget (Utilities|Array|Get(acopy) (LocalVariables|GetTargets%20) (LocalVariables|GetTargetIndex))))
      (bind _asbp_third_person_character_4 (Utilities|Casting|CastToBP_ThirdPersonCharacter _output_get_2))
      (Default|SetEnemyGuardVisible _asbp_third_person_character_4 true))))